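; BP_Cannon is a cannon actor that fires projectiles automatically on a repeating cycle from BeginPlay.
; After a FireRate delay it spawns a BP_Projectile at the ProjectileArrow's world location and rotation, scaled by ProjectileScale.
; CannonFireTimeline then animates the barrel's relative Y location, and its Cannon Fired Event track loops back to the delay for the next shot.
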(event EventBeginPlay
  (bind _projectilearrow (Variables|Default|GetProjectileArrow))
  (Utilities|FlowControl|Delay (Variables|CannonProperties|GetFireRate) :!label _label)
  (Game|SpawnActorfromClass "/Game/Blueprints/Actors/BP_Projectile.BP_Projectile_C" (Math|Transform|MakeTransform (Transformation|GetWorldLocation _projectilearrow) (Transformation|GetWorldRotation _projectilearrow) (Math|Conversions|ToVector(Float) (Variables|CannonProperties|GetProjectileScale))) "Undefined" 0 0)
  (bind _cannonbarrellocation (Timeline|CannonFireTimeline PlayFromStart)
    (:Update
      (Transformation|SetRelativeLocation (Variables|Default|GetCannonBarrel) (Math|Vector|MakeVector 0.0 _cannonbarrellocation 0.0) false false))
    (:CannonFiredEvent
      (goto _label))))

(event Collision|EventActorBeginOverlap
  (params (OtherActor :type Actor%20Object%20Reference)))

(event EventTick
  (params (DeltaSeconds :type Float%20%28single-precision%29)))

(fn ConstructionScript)