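; BP_Crystal is a pickup crystal with a light that is absorbed by the player on overlap.
; When the player pawn overlaps it, it caches its location, scale and light intensity, then plays DestroyCrystalTimeline.
; The timeline's separate tracks pull it toward the player's current position, shrink it to zero and fade the light.
; The actor destroys itself when the timeline finishes.
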(event EventBeginPlay)

(event Collision|EventActorBeginOverlap
  (params (OtherActor :type Actor%20Object%20Reference))
  (if (== OtherActor (Game|Player|GetPlayerPawn 0))
    (Variables|Default|SetLerpDestroyStartLocation (Transformation|GetActorLocation))
    (Variables|Default|SetStartScale (Transformation|GetActorScale3D))
    (Variables|Default|SetCrystalLightIntensity (Variables|/Script/Engine.LightComponentBase|GetIntensity (Variables|Default|GetCrystalLight)))
    (bind (_direction _destroylerpprogress _scale3dprogress _lightintensityprogress) (Timeline|DestroyCrystalTimeline Play)
      (:Update
        (Transformation|SetActorLocation (Math|Vector|Lerp(Vector) (Variables|Default|GetLerpDestroyStartLocation) (Transformation|GetActorLocation (Game|Player|GetPlayerPawn 0)) _destroylerpprogress) false false)
        (Transformation|SetActorScale3D (Math|Vector|Lerp(Vector) (Variables|Default|GetStartScale) "0, 0, 0" _scale3dprogress))
        (Rendering|Components|Light|SetIntensity (Variables|Default|GetCrystalLight) (Math|Float|Lerp (Variables|Default|GetCrystalLightIntensity) 0.0 _lightintensityprogress)))
      (:Finished
        (Actor|DestroyActor)))))

(event EventTick
  (params (DeltaSeconds :type Float%20%28single-precision%29)))

(fn ConstructionScript)